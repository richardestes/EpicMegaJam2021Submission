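; BP_MainGameMode is a game mode Blueprint that automatically respawns the player character after it is destroyed.
; On BeginPlay it binds to the OnDestroyed event of player 0's BP_PlayerCharacter.
; When that fires, it waits briefly, spawns a new BP_PlayerCharacter at the SpawnTransform variable and has player controller 0 possess it.
; The Respawn event then rebinds the destroy handler to the new pawn, so the cycle repeats.
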(event `Respawn`
  (bind _asbp_player_character (cast `/Game/Blueprints/Character/BP_PlayerCharacter` (`GameplayStatics.GetPlayerCharacter` 0) :!label _label))
  (add `self.OnDestroyed` _asbp_player_character (delegate `On Player Destroy`)))

(event `self.ReceiveBeginPlay`
  (goto _label))

(event `On Player Destroy` :!signature `self.OnDestroyed`
  (params (DestroyedActor :type "Actor Object Reference"))
  (`KismetSystemLibrary.Delay` 2.0)
  (bind _returnvalue (`|SpawnActorFromClass` "/Game/Blueprints/Character/BP_PlayerCharacter.BP_PlayerCharacter_C" (`self.Spawn Transform`) "Undefined" "OverrideRootScale" null false 0.0 "NewEnumerator0" "NewEnumerator0" true "NewEnumerator1" 150.0 140.0 375.0 600.0 375.0 325.0 "NewEnumerator1" 80.0 45.0 72.5 true 1.0 -40.0 40.0 5.0 475.0 0.06 false false false 10.0 1.0 250.0 "NewEnumerator0" false false false true 1.0 12.0 15.0 null))
  (`Controller.Possess` (`GameplayStatics.GetPlayerController` 0) _returnvalue)
  (`self.Respawn`))

(fn `UserConstructionScript`)