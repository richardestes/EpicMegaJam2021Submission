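; Spotlight actor that starts dark and fades in when the player enters its trigger box.
; BeginPlay applies the light color and sets the fade timeline's length from the Dim flag, overriding the earlier FadeDuration value.
; The box overlap plays the timeline to drive spotlight intensity.
; A DoOnce precedes the player cast, so the first overlap by any actor consumes the one-shot trigger.
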(event `self.ReceiveBeginPlay`
  (bind _fade_intensity (`self.Fade Intensity`))
  (`LightComponent.SetIntensity` (`self.SpotLight`) 0.0)
  (`TimelineComponent.SetTimelineLength` (`self.Fade Intensity`) (`self.Fade Duration`))
  (set `self.Activation Scale` (`self.Activation Scale`))
  (`LightComponent.SetLightColor` (`self.SpotLight`) (`self.Light Color`) true)
  (if (`self.Dim?`)
    (`TimelineComponent.SetTimelineLength` _fade_intensity 4.0)
    (else
      (`TimelineComponent.SetTimelineLength` _fade_intensity 10.0))))

(event `self.Box.OnComponentBeginOverlap`
  (params (OverlappedComponent :type "PrimitiveComponent Object Reference") (OtherActor :type "Actor Object Reference") (OtherComp :type "PrimitiveComponent Object Reference") (OtherBodyIndex :type Integer) (bFromSweep :type Boolean) (SweepResult :type "HitResult Structure (by ref)"))
  (`/Engine/EditorBlueprintResources/StandardMacros.DoOnce` false
    (:`Completed`
      (cast `/Game/Blueprints/Character/BP_PlayerCharacter` OtherActor)
      (bind (_direction _intensity) (`Timeline|Fade Intensity` :!via `PlayFromStart`)
        (:`Update`
          (`LightComponent.SetIntensity` (`self.SpotLight`) _intensity))))))

(fn `UserConstructionScript`)