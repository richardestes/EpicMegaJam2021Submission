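; BP_Respawn is a checkpoint actor that sets the player's respawn point when touched.
; When BP_PlayerCharacter overlaps the box, it writes the root's relative transform to SpawnTransform on BP_MainGameMode.
; It then applies the activated material to the mesh and shows the point light, which is hidden at BeginPlay.
; The construction script applies the configurable trigger transform, mesh transform and custom mesh.
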(event `self.ReceiveBeginPlay`
  (`SceneComponent.SetVisibility` (`self.PointLight`) false false))

(event `self.Box.OnComponentBeginOverlap`
  (params (OverlappedComponent :type "PrimitiveComponent Object Reference") (OtherActor :type "Actor Object Reference") (OtherComp :type "PrimitiveComponent Object Reference") (OtherBodyIndex :type Integer) (bFromSweep :type Boolean) (SweepResult :type "HitResult Structure (by ref)"))
  (cast `/Game/Blueprints/Character/BP_PlayerCharacter` OtherActor)
  (bind _asbp_main_game_mode (cast `/Game/Blueprints/GameMode/BP_MainGameMode` (`GameplayStatics.GetGameMode`)))
  (set `/Game/Blueprints/GameMode/BP_MainGameMode.Spawn Transform` (`SceneComponent.GetRelativeTransform` (`self.DefaultSceneRoot`)) _asbp_main_game_mode)
  (`PrimitiveComponent.SetMaterial` (`self.Respawn Mesh`) 0 (`self.Activated Material`))
  (`SceneComponent.SetVisibility` (`self.PointLight`) true false))

(fn `UserConstructionScript`
  (bind _respawn_mesh (`self.Respawn Mesh`))
  (bind _output_get (set `self.Spawn Trigger Size` (`self.Spawn Trigger Size`)))
  (`SceneComponent.K2_SetRelativeTransform` (`self.Box`) _output_get false false)
  (bind _output_get_2 (set `self.Mesh Transform` (`self.Mesh Transform`)))
  (`SceneComponent.K2_SetRelativeTransform` _respawn_mesh _output_get_2 false false)
  (`StaticMeshComponent.SetStaticMesh` _respawn_mesh (`self.Custom Respawn Mesh`)))