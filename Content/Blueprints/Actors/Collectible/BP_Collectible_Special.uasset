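; BP_Collectible_Special is a special pickup that flies into the player and adds one to the SpecialCollectibles count on BP_PlayerController.
; The construction script applies the configurable mesh, material and collision radius.
; On player overlap it stores its location and scale, then a timeline lerps it toward the player's current position while shrinking it to zero.
; When the timeline finishes, it increments the count and destroys itself after a brief delay.
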(event `self.ReceiveBeginPlay`
  (`SphereComponent.SetSphereRadius` (`self.Collision`) (`self.Collision Radius`) true)
  (bind _asbp_player_character (cast `/Game/Blueprints/Character/BP_PlayerCharacter` (`GameplayStatics.GetPlayerCharacter` 0)))
  (set `self.Player Ref` _asbp_player_character))

(event `self.ReceiveActorBeginOverlap`
  (params (OtherActor :type "Actor Object Reference"))
  (`/Game/Blueprints/Libraries/MacroLibrary.Is Player` OtherActor
    (:`IsPlayer`
      (`self.Store Starting Values`)
      (bind (_direction _collection_progress) (`Timeline|Collection Timeline` :!via `PlayFromStart`)
        (:`Update`
          (`self.Move To Player` _collection_progress)
          (`self.Scale Collectible` _collection_progress))
        (:`Finished`
          (bind _asbp_player_controller (cast `/Game/Blueprints/Character/BP_PlayerController` (`GameplayStatics.GetPlayerController` 0)))
          (`self.Pickup Collectible` _asbp_player_controller)
          (`KismetSystemLibrary.Delay` 0.2)
          (`self.K2_DestroyActor`))))))

(fn `Move To Player`
  (params (Alpha :type "Float (double-precision)"))
  (`self.K2_SetActorLocation` (`KismetMathLibrary.VLerp` (`self.Start Location`) (`self.K2_GetActorLocation` (`GameplayStatics.GetPlayerPawn` 0)) Alpha)))

(fn `Pickup Collectible`
  (params (`Player Controller` :type "PlayerController Object Reference"))
  (bind _asbp_player_controller (cast `/Game/Blueprints/Character/BP_PlayerController` `Player Controller`))
  (set `/Game/Blueprints/Character/BP_PlayerController.Special Collectibles` (+ (`/Game/Blueprints/Character/BP_PlayerController.Special Collectibles` _asbp_player_controller) 1) _asbp_player_controller))

(fn `Scale Collectible`
  (params (Alpha :type "Float (double-precision)"))
  (`self.SetActorScale3D` (`KismetMathLibrary.VLerp` (`self.Start Scale`) (0.0 0.0 0.0) Alpha)))

(fn `Store Starting Values`
  (set `self.Start Location` (`self.K2_GetActorLocation`))
  (set `self.Start Scale` (`self.GetActorScale3D`)))

(fn `UserConstructionScript`
  (`SphereComponent.SetSphereRadius` (`self.Collision`) (`self.Collision Radius`) true)
  (`PrimitiveComponent.SetMaterial` (`self.Mesh`) 0 (`self.Material Instance`))
  (bind _output_get (set `self.Custom Mesh` (`self.Custom Mesh`)))
  (`StaticMeshComponent.SetStaticMesh` (`self.Mesh`) _output_get))