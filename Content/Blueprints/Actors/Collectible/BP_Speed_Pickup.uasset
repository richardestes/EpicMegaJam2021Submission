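; Collectible speed-boost pickup that temporarily raises the player character's walk speed.
; When the player overlaps the sphere, a timeline pulls the pickup toward the pawn while shrinking it to zero.
; A second timeline then drives MaxWalkSpeed from its curve; after a configurable delay, speed resets to a hardcoded default and the actor destroys itself.
; The construction script applies a configurable mesh.
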(event `self.ReceiveBeginPlay`
  (`SphereComponent.SetSphereRadius` (`self.Sphere`) (`SphereComponent.SphereRadius` (`self.Sphere`)) true)
  (bind _asbp_player_character (cast `/Game/Blueprints/Character/BP_PlayerCharacter` (`GameplayStatics.GetPlayerCharacter` 0)))
  (set `self.Player Ref` _asbp_player_character))

(event `self.Sphere.OnComponentBeginOverlap`
  (params (OverlappedComponent :type "PrimitiveComponent Object Reference") (OtherActor :type "Actor Object Reference") (OtherComp :type "PrimitiveComponent Object Reference") (OtherBodyIndex :type Integer) (bFromSweep :type Boolean) (SweepResult :type "HitResult Structure (by ref)"))
  (bind _charactermovement (`Character.CharacterMovement` (`self.Player Ref`)))
  (if (== OtherActor (`self.Player Ref`))
    (`self.Store Starting Value`)
    (bind (_direction _collection_progress) (`Timeline|Move and Scale` :!via `PlayFromStart`)
      (:`Update`
        (`self.Move To Player` _collection_progress)
        (`self.Scale Collectible` _collection_progress))
      (:`Finished`
        (`/Engine/EditorBlueprintResources/StandardMacros.IsValid` (`self.Player Ref`)
          (:`Is Valid`
            (bind (_direction_2 _alpha) (`Timeline|Speed Up Movement` :!via `PlayFromStart`)
              (:`Update`
                (set `CharacterMovementComponent.MaxWalkSpeed` _alpha _charactermovement))
              (:`Finished`
                (`KismetSystemLibrary.Delay` (`self.Boost Cooldown Delay`) :!label _label)
                (set `CharacterMovementComponent.MaxWalkSpeed` 375.0 _charactermovement)
                (`KismetSystemLibrary.Delay` 1.0)
                (`self.K2_DestroyActor`))))
          (:`Is Not Valid`
            (goto _label)))))))

(fn `Move To Player`
  (params (Alpha :type "Float (double-precision)"))
  (`self.K2_SetActorLocation` (`KismetMathLibrary.VLerp` (`self.Start Location`) (`self.K2_GetActorLocation` (`GameplayStatics.GetPlayerPawn` 0)) Alpha)))

(fn `Scale Collectible`
  (params (Alpha :type "Float (double-precision)"))
  (`self.SetActorScale3D` (`KismetMathLibrary.VLerp` (`self.Start Scale`) (0.0 0.0 0.0) Alpha)))

(fn `Store Starting Value`
  (set `self.Start Location` (`self.K2_GetActorLocation`))
  (set `self.Start Scale` (`self.GetActorScale3D`)))

(fn `UserConstructionScript`
  (set `self.Material Instance` (`self.Material Instance`))
  (bind _output_get (set `self.Custom Mesh` (`self.Custom Mesh`)))
  (`StaticMeshComponent.SetStaticMesh` (`self.Mesh`) _output_get))