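; A platform actor that warns, then vanishes shortly after the player character enters its trigger box.
; The overlap swaps the floor to a danger material, then after a delay hides it and disables collision, either restoring it later or destroying the actor depending on Respawn.
; Ending any overlap also runs the delayed ResetProperties restore, without checking Respawn.
; The construction script applies a configurable floor scale.
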(event `self.Box.OnComponentBeginOverlap`
  (params (OverlappedComponent :type "PrimitiveComponent Object Reference") (OtherActor :type "Actor Object Reference") (OtherComp :type "PrimitiveComponent Object Reference") (OtherBodyIndex :type Integer) (bFromSweep :type Boolean) (SweepResult :type "HitResult Structure (by ref)"))
  (cast `/Game/Blueprints/Character/BP_PlayerCharacter` OtherActor)
  (`PrimitiveComponent.SetMaterial` (`self.Floor`) 0 "/Game/Locomotion/Demo/Materials/M_Blueprint_Dangerous.M_Blueprint_Dangerous")
  (`KismetSystemLibrary.Delay` (`self.Disappear Delay`))
  (`SceneComponent.SetVisibility` (`self.Floor`) false false)
  (`PrimitiveComponent.SetCollisionEnabled` (`self.Floor`) "NoCollision")
  (if (`self.Respawn?`)
    (`self.ResetProperties`)
    (else
      (`self.K2_DestroyActor`))))

(event `self.Box.OnComponentEndOverlap`
  (params (OverlappedComponent :type "PrimitiveComponent Object Reference") (OtherActor :type "Actor Object Reference") (OtherComp :type "PrimitiveComponent Object Reference") (OtherBodyIndex :type Integer))
  (`self.ResetProperties`))

(fn `UserConstructionScript`
  (`SceneComponent.SetRelativeScale3D` (`self.Floor`) (`self.Scale`)))