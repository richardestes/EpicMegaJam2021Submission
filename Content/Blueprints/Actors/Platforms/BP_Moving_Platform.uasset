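; Moving platform actor that travels from its starting location to a configurable end location while the player is inside its trigger box.
; Player overlap plays a Timeline that lerps the relative location after a delay, and leaving reverses it after the same delay.
; The Timeline's play rate is scaled by the configured duration.
; The construction script applies mesh, scale and rotation to the platform and a reference mesh placed at the end location.
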(event `self.ReceiveBeginPlay`
  (set `self.Start Location` (`SceneComponent.RelativeLocation` (`self.MainPlatform`))))

(event `self.Box.OnComponentBeginOverlap`
  (params (OverlappedComponent :type "PrimitiveComponent Object Reference") (OtherActor :type "Actor Object Reference") (OtherComp :type "PrimitiveComponent Object Reference") (OtherBodyIndex :type Integer) (bFromSweep :type Boolean) (SweepResult :type "HitResult Structure (by ref)"))
  (cast `/Game/Blueprints/Character/BP_PlayerCharacter` OtherActor)
  (`TimelineComponent.SetPlayRate` (`self.Move Platform`) (/ 1.0 (`self.Duration (Seconds)`)))
  (`KismetSystemLibrary.Delay` (`self.Delay Duration`))
  (bind (_direction _movetrack) (`Timeline|Move Platform` :!label _label)
    (:`Update`
      (`SceneComponent.K2_SetRelativeLocation` (`self.MainPlatform`) (`KismetMathLibrary.VLerp` (`self.Start Location`) (`self.End Location`) _movetrack) false false))))

(event `self.Box.OnComponentEndOverlap`
  (params (OverlappedComponent :type "PrimitiveComponent Object Reference") (OtherActor :type "Actor Object Reference") (OtherComp :type "PrimitiveComponent Object Reference") (OtherBodyIndex :type Integer))
  (cast `/Game/Blueprints/Character/BP_PlayerCharacter` OtherActor)
  (`TimelineComponent.SetPlayRate` (`self.Move Platform`) (/ 1.0 (`self.Duration (Seconds)`)))
  (`KismetSystemLibrary.Delay` (`self.Delay Duration`))
  (goto _label :!via `Reverse`))

(fn `UserConstructionScript`
  (bind _mainplatform (`self.MainPlatform`))
  (bind _end_platform_reference (`self.End Platform Reference`))
  (bind _end_location (`self.End Location`))
  (`StaticMeshComponent.SetStaticMesh` _mainplatform (`self.Platform Mesh`))
  (`StaticMeshComponent.SetStaticMesh` _end_platform_reference (`self.Platform Mesh`))
  (`SceneComponent.SetRelativeScale3D` _mainplatform (`self.Scale`))
  (`SceneComponent.SetRelativeScale3D` _end_platform_reference (`self.Scale`))
  (`SceneComponent.K2_SetRelativeLocation` _end_platform_reference _end_location false false)
  (`SceneComponent.K2_SetRelativeRotation` _mainplatform (`self.Rotation`) false false)
  (`SceneComponent.K2_SetRelativeRotation` _end_platform_reference (`self.Rotation`) false false)
  (`SceneComponent.K2_SetRelativeLocation` (`self.End Platform Reference`) _end_location false false))