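; DemoProjectile is a laser projectile actor in OpenSpaceAsteroid that plays a shot sound on spawn and damages what it hits.
; Its Trigger overlap reacts once, only to components that block WorldDynamic and do not belong to the instigator.
; A hit applies point damage, pushes physics bodies with a mass-scaled impulse, spawns a mesh-sized explosion with sound, then destroys itself.
; Effect locations fall back to the actor position when the sweep distance is zero.
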(event `self.ReceiveBeginPlay`
  (`GameplayStatics.PlaySoundAtLocation` "/Game/OpenSpaceAsteroid/Audio/Laser_Gun_Shot_Fast_Cue.Laser_Gun_Shot_Fast_Cue" (`self.K2_GetActorLocation`) (struct) 1.0 1.0 0.0 null null null))

(event `self.Trigger.OnComponentBeginOverlap`
  (params (OverlappedComponent :type "PrimitiveComponent Object Reference") (OtherActor :type "Actor Object Reference") (OtherComp :type "PrimitiveComponent Object Reference") (OtherBodyIndex :type Integer) (bFromSweep :type Boolean) (SweepResult :type "HitResult Structure (by ref)"))
  (bind (_bblockinghit _binitialoverlap _time _distance _location _impactpoint) (`GameplayStatics.BreakHitResult` SweepResult))
  (bind _returnvalue (`KismetMathLibrary.SelectVector` (`self.K2_GetActorLocation`) _impactpoint (== _distance 0.0)))
  (if (and (`|EnumEquality` (`PrimitiveComponent.GetCollisionResponseToChannel` OtherComp "ECC_WorldDynamic") "ECR_Block") (!= OtherActor (`self.Instigator`)))
    (`/Engine/EditorBlueprintResources/StandardMacros.DoOnce` false
      (:`Completed`
        (if (`SceneComponent.IsSimulatingPhysics` OtherComp "None")
          (`PrimitiveComponent.AddImpulseAtLocation` OtherComp (* (`self.GetActorForwardVector`) (* (`PrimitiveComponent.GetMass` OtherComp) 1000.0)) _returnvalue "None"))
        (`GameplayStatics.ApplyPointDamage` OtherActor 1.0 (`self.GetActorForwardVector`) SweepResult (`self.GetInstigatorController`) self)
        (`GameplayStatics.SpawnEmitterAtLocation` "/Game/OpenSpaceAsteroid/Particles/P_Explosion.P_Explosion" _returnvalue (`KismetMathLibrary.RandomRotator` true) (`KismetMathLibrary.Conv_DoubleToVector` (* (`.SphereRadius` (`KismetSystemLibrary.GetComponentBounds` (`self.Mesh_Projectile`))) 0.02)))
        (`GameplayStatics.PlaySoundAtLocation` "/Game/OpenSpaceAsteroid/Audio/Hit_Cue.Hit_Cue" _returnvalue (struct) 1.0 1.0 0.0 null null null)
        (`self.K2_DestroyActor`)))))

(fn `UserConstructionScript`)