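; DemoFighter is a player-controlled physics fighter craft that flies and fires projectiles.
; Each tick, WASD flags drive acceleration-based force on the Hull along forward and right, while axis inputs apply local-space pitch and yaw torque.
; Roll is gradually lerped back to level every tick.
; Holding left mouse runs a Gate and Delay loop that repeatedly spawns DemoProjectile pairs from either side of the craft.
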(event `self.ReceiveTick`
  (params (DeltaSeconds :type "Float (single-precision)"))
  (bind _returnvalue (`self.K2_GetActorRotation`))
  (bind _hull (`self.Hull`))
  (`PrimitiveComponent.AddForce` _hull (* (+ (* (`self.GetActorForwardVector`) (`self.AxisForward`)) (* (`self.GetActorRightVector`) (`self.AxisRight`))) (`self.Speed`)) "None" true)
  (`PrimitiveComponent.AddTorqueInDegrees` _hull (* (`KismetMathLibrary.TransformDirection` (`self.GetTransform`) (`KismetMathLibrary.MakeVector` 0.0 (* (`self.GetInputAxisKeyValue`) -1.0) (`self.GetInputAxisKeyValue`))) 100.0) "None" true)
  (`self.K2_SetActorRotation` (`KismetMathLibrary.RLerp` _returnvalue (`KismetMathLibrary.MakeRotator` 0.0 (.pitch _returnvalue) (.yaw _returnvalue)) 0.02 true)))

(event `Key|W`
  (params (Key :type "Key Structure"))
  (:`Pressed`
    (set `self.AxisForward` 1.0))
  (:`Released`
    (set `self.AxisForward` 0.0)))

(event `Key|D`
  (params (Key :type "Key Structure"))
  (:`Pressed`
    (set `self.AxisRight` 1.0))
  (:`Released`
    (set `self.AxisRight` 0.0)))

(event `Key|S`
  (params (Key :type "Key Structure"))
  (:`Pressed`
    (set `self.AxisForward` -1.0))
  (:`Released`
    (set `self.AxisForward` 0.0)))

(event `Key|A`
  (params (Key :type "Key Structure"))
  (:`Pressed`
    (set `self.AxisRight` -1.0))
  (:`Released`
    (set `self.AxisRight` 0.0)))

(event `Key|LeftMouseButton`
  (params (Key :type "Key Structure"))
  (bind _returnvalue (`self.GetTransform`))
  (:`Pressed`
    (`|ExecutionSequence`
      (:`then_0`
        (goto _label :!via `Open`))
      (:`then_1`
        (`/Engine/EditorBlueprintResources/StandardMacros.Gate` true :!label _label
          (:`Exit`
            (`|SpawnActorFromClass` "/Game/OpenSpaceAsteroid/Blueprints/DemoProjectile.DemoProjectile_C" (`KismetMathLibrary.ComposeTransforms` (`KismetMathLibrary.Conv_VectorToTransform` (0.0 -300.0 0.0)) _returnvalue) "Undefined" "OverrideRootScale" null self)
            (`|SpawnActorFromClass` "/Game/OpenSpaceAsteroid/Blueprints/DemoProjectile.DemoProjectile_C" (`KismetMathLibrary.ComposeTransforms` (`KismetMathLibrary.Conv_VectorToTransform` (0.0 300.0 0.0)) _returnvalue) "Undefined" "OverrideRootScale" null self)
            (`KismetSystemLibrary.Delay` 0.15)
            (goto _label))))))
  (:`Released`
    (goto _label :!via `Close`)))

(fn `UserConstructionScript`)